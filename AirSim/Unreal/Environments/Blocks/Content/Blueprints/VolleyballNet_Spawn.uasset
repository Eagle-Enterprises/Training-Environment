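; Spawner Blueprint that places a VN actor, apparently the volleyball net, in the level at runtime.
; A DoOnce on Tick triggers the spawn routine, which first creates four TargetPoints, all at the same hard-coded transform.
; It then gathers every TargetPoint in the level and spawns VN at a random one, so other TargetPoints are also candidates.
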(event `self.ReceiveTick`
  (params (DeltaSeconds :type "Float (single-precision)"))
  (`/Engine/EditorBlueprintResources/StandardMacros.DoOnce` false
    (:`Completed`
      (`self.VolleyballNet_Spawn`))))

(event `VolleyballNet_Spawn`
  (`|SpawnActorFromClass` "/Script/Engine.TargetPoint" (`KismetMathLibrary.MakeTransform` (-450.0 1950.0 30.0)) "Undefined" "OverrideRootScale" null null)
  (`|SpawnActorFromClass` "/Script/Engine.TargetPoint" (`KismetMathLibrary.MakeTransform` (-450.0 1950.0 30.0)) "Undefined" "OverrideRootScale" null null)
  (`|SpawnActorFromClass` "/Script/Engine.TargetPoint" (`KismetMathLibrary.MakeTransform` (-450.0 1950.0 30.0)) "Undefined" "OverrideRootScale" null null)
  (`|SpawnActorFromClass` "/Script/Engine.TargetPoint" (`KismetMathLibrary.MakeTransform` (-450.0 1950.0 30.0)) "Undefined" "OverrideRootScale" null null)
  (bind _outactors (`GameplayStatics.GetAllActorsOfClass` "/Script/Engine.TargetPoint"))
  (bind _output_get (set `self.Out Actors` _outactors))
  (`|SpawnActorFromClass` "/Game/Blueprints/VN.VN_C" (`self.GetTransform` (`KismetArrayLibrary.Array_Random` _output_get)) "Undefined" "OverrideRootScale" null null))

(fn `UserConstructionScript`)