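; GPS_MoveToCoordinate is a Blueprint that sends the player controller to a coordinate stored in the game instance, apparently for UAV movement.
; Every tick, MoveUAVTo reads BP_Demo1_Instance and calls SimpleMoveToLocation with a truncated goal at Z zero.
; The X entry feeds both goal axes, so the Y entry is unused.
; Disconnected nodes hold a Y assignment and empty-value debug checks.
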(event Custom|Move%20UAV%20To
  (bind _asbp_demo_1_instance (Utilities|Casting|CastToBP_Demo1_Instance (Game|GetGameInstance)))
  (bind _output_get (Variables|/Game/Blueprints/BP_Demo1_Instance.BP_Demo1_Instance_C|SetPlayer_Enter_X_Coordinate _asbp_demo_1_instance (Variables|/Game/Blueprints/BP_Demo1_Instance.BP_Demo1_Instance_C|GetPlayer_Enter_X_Coordinate _asbp_demo_1_instance)))
  (AI|Navigation|SimpleMovetoLocation (Game|GetPlayerController 0) (Math|Vector|MakeVector (Math|Conversions|ToFloat(Integer) (Math|Float|Truncate _output_get)) (Math|Conversions|ToFloat(Integer) (Math|Float|Truncate (stale _output_get))) 0.0)))

(event EventTick
  (params (DeltaSeconds :type Float%20%28single-precision%29))
  (CallFunction|MoveUAVto))

(fn ConstructionScript)