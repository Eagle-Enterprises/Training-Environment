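; BP_Opponent_Random_Asset spawns test props at hard-coded world locations and randomly selects one of them.
; BeginPlay spawns five StaticMeshActors, setting meshes from a reassigned AssetMesh variable, plus a BP_Asset_Actor, then adds a random pick to the "asset" layer.
; All six remain spawned, and separate random rolls drive the debug print and Tick's per-frame player-distance readout, so neither necessarily matches the layered actor.
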(event `self.ReceiveBeginPlay`
  (bind _actorlayer (make `ActorLayer` "asset"))
  (bind _returnvalue (`|SpawnActorFromClass` "/Script/Engine.StaticMeshActor" (`KismetMathLibrary.MakeTransform` (2483.0 1980.0 3970.0)) "AlwaysSpawn" "OverrideRootScale" null null))
  (`StaticMeshComponent.SetStaticMesh` (`StaticMeshActor.StaticMeshComponent` _returnvalue) (stale _output_get))
  (bind _output_get (set `self.Asset Mesh` "/Game/Enemy_Assets/SM_Cone.SM_Cone"))
  (bind _returnvalue_2 (`|SpawnActorFromClass` "/Script/Engine.StaticMeshActor" (`KismetMathLibrary.MakeTransform` (2483.0 1980.0 4180.0)) "AlwaysSpawn" "OverrideRootScale" null null))
  (`StaticMeshComponent.SetStaticMesh` (`StaticMeshActor.StaticMeshComponent` _returnvalue_2) (stale _output_get_2))
  (bind _output_get_2 (set `self.Asset Mesh` "/Game/Enemy_Assets/SM_Cube.SM_Cube"))
  (bind _returnvalue_3 (`|SpawnActorFromClass` "/Script/Engine.StaticMeshActor" (`KismetMathLibrary.MakeTransform` (2483.0 1980.0 3970.0)) "AlwaysSpawn" "OverrideRootScale" null null))
  (`StaticMeshComponent.SetStaticMesh` (`StaticMeshActor.StaticMeshComponent` _returnvalue_3) (stale _output_get_3))
  (bind _output_get_3 (set `self.Asset Mesh` "/Game/Enemy_Assets/SM_Football.SM_Football"))
  (bind _returnvalue_4 (`|SpawnActorFromClass` "/Script/Engine.StaticMeshActor" (`KismetMathLibrary.MakeTransform` (2483.0 1980.0 3970.0)) "AlwaysSpawn" "OverrideRootScale" null null))
  (`StaticMeshComponent.SetStaticMesh` (`StaticMeshActor.StaticMeshComponent` _returnvalue_4) (stale _output_get_4))
  (bind _output_get_4 (set `self.Asset Mesh` "/Game/Enemy_Assets/SM_Sphere.SM_Sphere"))
  (bind _returnvalue_5 (`|SpawnActorFromClass` "/Script/Engine.StaticMeshActor" (`KismetMathLibrary.MakeTransform` (2483.0 1980.0 3970.0)) "AdjustIfPossibleButAlwaysSpawn" "OverrideRootScale" null null))
  (`StaticMeshComponent.SetStaticMesh` (`StaticMeshActor.StaticMeshComponent` _returnvalue_5) (stale _output_get_5))
  (bind _output_get_5 (set `self.Asset Mesh` "/Game/Enemy_Assets/SM_Cone.SM_Cone"))
  (bind _returnvalue_6 (`|SpawnActorFromClass` "/Game/EE_Asset_Model/BP_Asset_Actor.BP_Asset_Actor_C" (`KismetMathLibrary.MakeTransform` (2483.0 1980.0 3970.0)) "AlwaysSpawn" "OverrideRootScale" null null))
  (bind _output (`|GetArrayItem` (`|MakeArray` _returnvalue _returnvalue_2 _returnvalue_3 _returnvalue_4 _returnvalue_5 _returnvalue_6 :!type "Actor Object Reference") (`KismetMathLibrary.RandomIntegerInRange` 0 5)))
  (bind _output_get_6 (set `self.NewVar_0` _output))
  (`LayersBlueprintLibrary.AddActorToLayer` _output_get_6 _actorlayer)
  (bind _returnvalue_7 (`LayersBlueprintLibrary.GetActors` _actorlayer))
  (`GameplayStatics.GetActorArrayAverageLocation` _returnvalue_7)
  (`KismetSystemLibrary.PrintString` (`KismetStringLibrary.Conv_ObjectToString` _output) true true (struct :`R` 1.0 :`B` 0.806712 :`A` 1.0) 50.0))

(event `self.ReceiveTick`
  (params (DeltaSeconds :type "Float (single-precision)"))
  (`KismetSystemLibrary.PrintString` (`KismetStringLibrary.Conv_DoubleToString` (`Actor.GetDistanceTo` (`GameplayStatics.GetPlayerPawn` 0) (`|GetArrayItem` (`|MakeArray` (stale `self.ReceiveBeginPlay` _returnvalue) (stale `self.ReceiveBeginPlay` _returnvalue_2) (stale `self.ReceiveBeginPlay` _returnvalue_3) (stale `self.ReceiveBeginPlay` _returnvalue_4) (stale `self.ReceiveBeginPlay` _returnvalue_5) (stale `self.ReceiveBeginPlay` _returnvalue_6) :!type "Actor Object Reference") (`KismetMathLibrary.RandomIntegerInRange` 0 5)))) true true (struct :`G` 0.66 :`B` 1.0 :`A` 1.0) DeltaSeconds))