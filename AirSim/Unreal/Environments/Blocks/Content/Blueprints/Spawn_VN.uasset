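; Spawn_VN is a spawner Blueprint that places one VN actor at a randomly chosen point in the level.
; On its first Tick, a DoOnce calls a test event that spawns four TargetPoints at hardcoded locations.
; It then gathers every TargetPoint in the world, including any already placed, and spawns VN at the transform of a random one.
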(event `self.ReceiveTick`
  (params (DeltaSeconds :type "Float (single-precision)"))
  (`/Engine/EditorBlueprintResources/StandardMacros.DoOnce` false
    (:`Completed`
      (`self.test1`))))

(event `test1`
  (`|SpawnActorFromClass` "/Script/Engine.TargetPoint" (`KismetMathLibrary.MakeTransform` (24060.0 790.0 3970.0)) "Undefined" "OverrideRootScale" null null)
  (`|SpawnActorFromClass` "/Script/Engine.TargetPoint" (`KismetMathLibrary.MakeTransform` (22270.0 790.0 4000.0)) "Undefined" "OverrideRootScale" null null)
  (`|SpawnActorFromClass` "/Script/Engine.TargetPoint" (`KismetMathLibrary.MakeTransform` (22270.0 2860.0 4000.0)) "Undefined" "OverrideRootScale" null null)
  (`|SpawnActorFromClass` "/Script/Engine.TargetPoint" (`KismetMathLibrary.MakeTransform` (24240.0 2860.0 4000.0)) "Undefined" "OverrideRootScale" null null)
  (bind _outactors (`GameplayStatics.GetAllActorsOfClass` "/Script/Engine.TargetPoint"))
  (bind _output_get (set `self.Arrray of Actors` _outactors))
  (`|SpawnActorFromClass` "/Game/Blueprints/VN.VN_C" (`self.GetTransform` (`KismetArrayLibrary.Array_Random` _output_get)) "Undefined" "OverrideRootScale" null null))

(fn `UserConstructionScript`)