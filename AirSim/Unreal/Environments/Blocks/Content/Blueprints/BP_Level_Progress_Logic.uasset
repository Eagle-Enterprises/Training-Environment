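; BP_Level_Progress_Logic drives the demo's advancement loop through a completion counter kept in BP_Demo1_Instance, the Game Instance.
; On BeginPlay it spawns a BP_Level_Progress_Actor at the origin and caches one of its values as integer text.
; EndStateReached increments the counter and opens FlyingExampleMap, so progress survives level loads.
; Once the counter equals three, it instead shows the demo-complete screen, pauses the game and hides the cursor.
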(event `self.ReceiveBeginPlay`
  (bind _returnvalue (`|SpawnActorFromClass` "/Game/Blueprints/BP_Level_Progress_Actor.BP_Level_Progress_Actor_C" (`KismetMathLibrary.Conv_VectorToTransform` (0.0 0.0 0.0)) "Undefined" "OverrideRootScale" null null))
  (set `self.Actor Spawned` _returnvalue)
  (set `self.TextOutput` (`KismetTextLibrary.Conv_IntToText` (`KismetMathLibrary.FTrunc` (`/Game/Blueprints/BP_Level_Progress_Actor.NewVar_0` (`self.Actor Spawned`))))))

(event `End State Reached`
  ;[1 1 1] Game Advancement Loop
  (bind _asbp_demo_1_instance (cast `/Game/Blueprints/BP_Demo1_Instance` (`GameplayStatics.GetGameInstance`)))
  (bind _democomplete (`/Game/Blueprints/BP_Demo1_Instance.DemoComplete` _asbp_demo_1_instance))
  (if (== _democomplete 3)
    (bind _returnvalue (`|CreateWidget` "/Game/Blueprints/BP_Demo_Complete_Screen.BP_Demo_Complete_Screen_C"))
    (`UserWidget.AddToViewport` _returnvalue 0)
    (`GameplayStatics.SetGamePaused` true)
    (set `PlayerController.bShowMouseCursor` false (`GameplayStatics.GetPlayerController` 0))
    (else
      (set `/Game/Blueprints/BP_Demo1_Instance.DemoComplete` (+ _democomplete 1) _asbp_demo_1_instance)
      (`GameplayStatics.OpenLevelBySoftObjectPtr` "/Game/Maps/FlyingExampleMap.FlyingExampleMap"))))