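; BP_Demo1_Instance holds shared state for Demo 1, which appears to be a UAV and IED scenario, likely as a Game Instance.
; Its variables cover timing, IED count, player entry and target asset coordinates, FOB and obstacle spawn locations, UAV speed and UWB distance.
; ResetToDefault provides a clean restart by clearing these values, while setting DemoComplete to 1 rather than zero.
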(fn `ResetToDefault`
  ;[1 1 1] Clean Restart
  (set `self.Total Time` (struct))
  (set `self.IED's` 0)
  (set `self.InstanceTime` (struct))
  (set `self.DemoComplete` 1)
  (set `self.Player_Enter_X_Coordinate` 0.0)
  (set `self.Player_Enter_Y_Coordinate` 0.0)
  (set `self.Target_Asset_X_Coordinate` 0.0)
  (set `self.Target_Asset_Y_Coordinate` 0.0)
  (set `self.TargetAsset` null)
  (set `self.FOB_Location` (0.0 0.0 0.0))
  (set `self.UAV_Speed` 0.0)
  (set `self.Obstacle_Spawn_Location` (0.0 0.0 0.0))
  (set `self.UWBDistance` 0.0))