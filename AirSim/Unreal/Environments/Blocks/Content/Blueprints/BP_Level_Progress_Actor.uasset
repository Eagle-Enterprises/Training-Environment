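; BP_Level_Progress_Actor is a level actor that takes player input for pausing and level progression, enabling input on BeginPlay.
; D-Pad Down flip-flops a BP_Menu widget, game pause and the mouse cursor on and off.
; D-Pad Right increments DemoComplete on BP_Demo1_Instance and opens FlyingExampleMap.
; OnReset restores NewVar0 from the class defaults and prints a debug message.
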(event `self.K2_OnReset`
  (set `self.NewVar_0` (defaults `Object` (`GameplayStatics.GetObjectClass` self)))
  (`KismetSystemLibrary.PrintString` "On Reset was Called"))

(event `self.ReceiveBeginPlay`
  (`self.EnableInput` (`GameplayStatics.GetPlayerController` 0)))

(event `Key|Gamepad_DPad_Down` :consume false :paused true
  (params (Key :type "Key Structure"))
  (bind _returnvalue (`GameplayStatics.GetPlayerController` 0))
  ;[1 1 1] Pause Game
  (:`Pressed`
    (`/Engine/EditorBlueprintResources/StandardMacros.FlipFlop`
      (:`A`
        (bind _returnvalue_2 (`|CreateWidget` "/Game/Blueprints/BP_Menu.BP_Menu_C"))
        (`UserWidget.AddToViewport` _returnvalue_2 0)
        (`GameplayStatics.SetGamePaused` true)
        (set `PlayerController.bShowMouseCursor` true _returnvalue))
      (:`B`
        (`Widget.RemoveFromParent` _returnvalue_2)
        (`GameplayStatics.SetGamePaused` false)
        (set `PlayerController.bShowMouseCursor` false _returnvalue)))))

(event `Key|Gamepad_DPad_Right`
  (params (Key :type "Key Structure"))
  (:`Pressed`
    (bind _asbp_demo_1_instance (cast `/Game/Blueprints/BP_Demo1_Instance` (`GameplayStatics.GetGameInstance`)))
    (set `/Game/Blueprints/BP_Demo1_Instance.DemoComplete` (+ (`/Game/Blueprints/BP_Demo1_Instance.DemoComplete` _asbp_demo_1_instance) 1) _asbp_demo_1_instance)
    (`GameplayStatics.OpenLevelBySoftObjectPtr` "/Game/Maps/FlyingExampleMap.FlyingExampleMap")))

(fn `UserConstructionScript`)