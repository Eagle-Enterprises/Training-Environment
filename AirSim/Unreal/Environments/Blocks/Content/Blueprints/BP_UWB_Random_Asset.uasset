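; Blueprint that picks a random target asset for the UWB demo and tracks the player's distance to it.
; On first Tick, a DoOnce runs OnPlayStart, which spawns BP_Asset_Actors at fixed locations, stores a random one as TargetAsset in BP_Demo1_Instance and prints its name.
; Every Tick writes the player pawn's distance to that target into the game instance's UWBDistance.
; An archived custom event holds an older random mesh-placement approach.
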(event `On Play Start`
  ;[1 1 1] Spawn EE Assets
  (bind _returnvalue (`|SpawnActorFromClass` "/Game/EE_Asset_Model/BP_Asset_Actor.BP_Asset_Actor_C" (`KismetMathLibrary.MakeTransform` (-4660.0 -1540.0 20.0)) "AlwaysSpawn" "OverrideRootScale" null null))
  (bind _returnvalue_2 (`|SpawnActorFromClass` "/Game/EE_Asset_Model/BP_Asset_Actor.BP_Asset_Actor_C" (`KismetMathLibrary.MakeTransform` (-4890.0 -540.0 20.0)) "AlwaysSpawn" "OverrideRootScale" null null))
  (bind _returnvalue_3 (`|SpawnActorFromClass` "/Game/EE_Asset_Model/BP_Asset_Actor.BP_Asset_Actor_C" (`KismetMathLibrary.MakeTransform` (-2170.0 2460.0 30.0)) "AlwaysSpawn" "OverrideRootScale" null null))
  (bind _returnvalue_4 (`|SpawnActorFromClass` "/Game/EE_Asset_Model/BP_Asset_Actor.BP_Asset_Actor_C" (`KismetMathLibrary.MakeTransform` (-410.0 1950.0 40.0)) "AlwaysSpawn" "OverrideRootScale" null null))
  (bind _returnvalue_5 (`|SpawnActorFromClass` "/Game/EE_Asset_Model/BP_Asset_Actor.BP_Asset_Actor_C" (`KismetMathLibrary.MakeTransform` (-4660.0 510.0 40.0)) "AlwaysSpawn" "OverrideRootScale" null null))
  (bind _returnvalue_6 (`|SpawnActorFromClass` "/Game/EE_Asset_Model/BP_Asset_Actor.BP_Asset_Actor_C" (`KismetMathLibrary.MakeTransform` (-3900.0 1850.0 -50.0)) "AlwaysSpawn" "OverrideRootScale" null null))
  (bind _asbp_demo_1_instance (cast `/Game/Blueprints/BP_Demo1_Instance` (`GameplayStatics.GetGameInstance`)))
  (bind _output_get (set `/Game/Blueprints/BP_Demo1_Instance.TargetAsset` (`|GetArrayItem` (`|MakeArray` _returnvalue _returnvalue_2 _returnvalue_3 _returnvalue_4 _returnvalue_5 _returnvalue_6 :!type "Actor Object Reference") (`KismetMathLibrary.RandomIntegerInRange` 0 5)) _asbp_demo_1_instance))
  (`KismetSystemLibrary.PrintString` (`KismetSystemLibrary.GetDisplayName` _output_get) true true (struct :`R` 1.0 :`B` 0.806712 :`A` 1.0) 50.0))

(event `self.ReceiveTick`
  (params (DeltaSeconds :type "Float (single-precision)"))
  (bind _asbp_demo_1_instance (cast `/Game/Blueprints/BP_Demo1_Instance` (`GameplayStatics.GetGameInstance`)))
  (set `/Game/Blueprints/BP_Demo1_Instance.UWBDistance` (`Actor.GetDistanceTo` (`GameplayStatics.GetPlayerPawn` 0) (`/Game/Blueprints/BP_Demo1_Instance.TargetAsset` _asbp_demo_1_instance)) _asbp_demo_1_instance)
  (`/Engine/EditorBlueprintResources/StandardMacros.DoOnce` false
    (:`Completed`
      (`self.On Play Start`))))

(event `CustomEvent`
  ;[1 1 1] ARCHIVE
  (bind _returnvalue (`|SpawnActorFromClass` "/Script/Engine.StaticMeshActor" (`KismetMathLibrary.MakeTransform` (0.0 0.0 0.0)) "AlwaysSpawn" "OverrideRootScale" null null))
  (`StaticMeshComponent.SetStaticMesh` (`StaticMeshActor.StaticMeshComponent` _returnvalue) (stale _output_get))
  (bind _output_get (set `self.Asset Mesh` "/Game/EE_Asset_Model/SM_Merged_Asset.SM_Merged_Asset"))
  (bind _outactors (`GameplayStatics.GetAllActorsOfClass` "/Game/EE_Asset_Model/BP_Asset_Actor.BP_Asset_Actor_C"))
  (`Actor.K2_SetActorLocation` _returnvalue (`Actor.K2_GetActorLocation` (`KismetArrayLibrary.Array_Random` _outactors)) false false))